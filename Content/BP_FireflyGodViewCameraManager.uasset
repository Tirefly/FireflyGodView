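; BP_FireflyGodViewCameraManager is a player camera manager that drives a god-view camera from a GodViewConfig.
; InitializeFor seeds PreviousLocation from either the configured initial location or the player controller's focal location, when the config is valid.
; BlueprintUpdateCamera fully overrides the view, taking location from CalcCameraLocation, which is defined outside this graph, with fixed rotation and FOV from the config.
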(event `self.ReceiveInitializeFor`
  (params (PC :type "PlayerController Object Reference"))
  (bind _godviewconfig (`self.GodViewConfig`)
    (:`then`
      (if (`FireflyGodViewConfig.bEnableCameraInitialLocation` _godviewconfig)
        (set `self.PreviousLocation` (`FireflyGodViewConfig.CameraInitialLocation` (`self.GodViewConfig`)))
        (else
          (set `self.PreviousLocation` (`PlayerController.GetFocalLocation` PC)))))
    (:`else`)))

(fn `BlueprintUpdateCamera`
  (params (CameraTarget :type "Actor Object Reference"))
  (returns (NewCameraLocation :type "Vector Structure") (NewCameraRotation :type "Rotator Structure") (NewCameraFOV :type "Float (single-precision)") (ReturnValue :type Boolean))
  (locals (OutLocation :type "Vector Structure"))
  (return (`self.CalcCameraLocation`) (`FireflyGodViewConfig.CameraInitialRotation` (`self.GodViewConfig`)) (`FireflyGodViewConfig.GodViewFOV` (`self.GodViewConfig`)) true))

(fn `UserConstructionScript`)